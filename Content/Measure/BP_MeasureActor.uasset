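; Measurement actor that holds points on a spline and shows them through an on-screen widget.
; CreateWidget spawns the widget and initializes it with a display unit and centimeter scale.
; Each Tick, once the spline has more than one point, it passes all world-space point locations to the widget, which is removed on EndPlay.
; SetFirstLocation positions a spline point, while the add and set-last location events are empty stubs.
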(event `self.ReceiveBeginPlay`)

(event `self.ReceiveTick`
  (params (DeltaSeconds :type "Float (single-precision)"))
  (if (> (`SplineComponent.GetNumberOfSplinePoints` (`self.Spline`)) 1)
    (message `/MyCustomWidget/Measure/BPI_MesureWidget.Update` (`self.MesureWidget`) (`self.Get Spline Locations`))))

(event `SetFirstLocation`
  (params (LocationWS :type "Vector Structure"))
  (`SplineComponent.SetLocationAtSplinePoint` (`self.Spline`) 0 LocationWS "World" true))

(event `AddLoacation`
  (params (LocationWS :type "Vector Structure")))

(event `SetLastLocation`
  (params (LocationWS :type "Vector Structure")))

(event `self.ReceiveEndPlay`
  (params (EndPlayReason :type "EEndPlayReason Enum" :default "Destroyed"))
  (`Widget.RemoveFromParent` (`self.MesureWidget`)))

(fn `CreateWidget`
  (params (Unit :type Text) (UnitScaleToCm :type "Float (double-precision)"))
  (bind _returnvalue (`|CreateWidget` (`self.WidgetClass`)))
  (bind _output_get (set `self.MesureWidget` _returnvalue))
  (message `/MyCustomWidget/Measure/BPI_MesureWidget.Init` _output_get Unit UnitScaleToCm)
  (`UserWidget.AddToViewport` _output_get 0))

(fn `Get Spline Locations`
  (returns (OutLocations :type "Array of Vector Structure"))
  (locals (Locations :type "Array of Vector Structure"))
  (bind _spline (`self.Spline`))
  (for _index (range (`SplineComponent.GetNumberOfSplinePoints` _spline))
    (`KismetArrayLibrary.Array_Add` (`local.Locations`) (`SplineComponent.GetLocationAtSplinePoint` _spline _index "World")))
  (return (`local.Locations`)))

(fn `UserConstructionScript`)