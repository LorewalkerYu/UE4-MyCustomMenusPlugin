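; BP_MesureManager runs the mouse-driven measuring tool, switching between linear and area (Square) measurement.
; StartMeasure destroys the current measure actor, spawns the matching linear or area actor and updates the pawn's state message.
; Left-mouse events from BP_Pawn feed cursor Visibility traces to that actor.
; Linear drags from press to release with Tick updating the end point, while Square adds a point on each release.
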(event `self.ReceiveBeginPlay`
  (`self.BindLeftMouse`))

(event `self.ReceiveTick`
  (params (DeltaSeconds :type "Float (single-precision)"))
  (switch `/MyCustomWidget/Measure/BPE_MeasureType` (`self.CurrentType`)
    (:`NewEnumerator1`
      (if (`self.StartTick`)
        (bind (_hit_result_blocking_hit _hit_result_location) (`self.CursorHit`))
        (if _hit_result_blocking_hit
          (`self.SetLast` _hit_result_location))))))

(event `StartMeasure`
  (params (Type :type "/MyCustomWidget/Measure/BPE_MeasureType Enum" :default "NewEnumerator0"))
  (`self.ProcessType` Type)
  (set `self.CurrentType` Type))

(event `SetFirst`
  (params (LocationWS :type "Vector Structure"))
  (bind _mesureactor (`self.MesureActor`))
  (`/Engine/EditorBlueprintResources/StandardMacros.IsValid` _mesureactor
    (:`Is Valid`
      (`/MyCustomWidget/Measure/BP_MeasureActor.SetFirstLocation` _mesureactor LocationWS))))

(event `AddLocation`
  (params (LocationWS :type "Vector Structure"))
  (bind _mesureactor (`self.MesureActor`))
  (`/Engine/EditorBlueprintResources/StandardMacros.IsValid` _mesureactor
    (:`Is Valid`
      (`/MyCustomWidget/Measure/BP_MeasureActor.AddLoacation` _mesureactor LocationWS))))

(event `SetLast`
  (params (LocationWS :type "Vector Structure"))
  (bind _mesureactor (`self.MesureActor`))
  (`/Engine/EditorBlueprintResources/StandardMacros.IsValid` _mesureactor
    (:`Is Valid`
      (`/MyCustomWidget/Measure/BP_MeasureActor.SetLastLocation` _mesureactor LocationWS))))

(event `BindLeftMouse`
  (bind _asbp_pawn (cast `/Game/Blueprints/Frame/BP_Pawn` (`GameplayStatics.GetPlayerPawn` 0)))
  (add `/Game/Blueprints/Frame/BP_Pawn.LeftMouseButton` _asbp_pawn (delegate `CustomEvent_0`)))

(event `CustomEvent_0`
  (params (InputEvent :type "EInputEvent Enum" :default "IE_Pressed"))
  (switch `EInputEvent` InputEvent
    (:`IE_Pressed`
      (switch `/MyCustomWidget/Measure/BPE_MeasureType` (`self.CurrentType`)
        (:`NewEnumerator1`
          (bind (_hit_result_blocking_hit _hit_result_location) (`self.CursorHit`))
          (if _hit_result_blocking_hit
            (`self.SetFirst` _hit_result_location)
            (`self.AddLocation` _hit_result_location)
            (set `self.StartTick` true)))))
    (:`IE_Released`
      (switch `/MyCustomWidget/Measure/BPE_MeasureType` (`self.CurrentType`)
        (:`NewEnumerator0`
          (set `self.StartTick` false :!label _label))
        (:`NewEnumerator1`
          (goto _label))
        (:`NewEnumerator2`
          (bind (_hit_result_blocking_hit_2 _hit_result_location_2) (`self.CursorHit`))
          (if _hit_result_blocking_hit_2
            (`self.AddLocation` _hit_result_location_2)))))))

(fn `CursorHit`
  (returns (`Hit Result Blocking Hit` :type Boolean) (`Hit Result Location` :type "Vector Structure"))
  (bind _hitresult (`PlayerController.GetHitResultUnderCursorByChannel` (`GameplayStatics.GetPlayerController` 0) "TraceTypeQuery1" true))
  (return (`GameplayStatics.BreakHitResult` _hitresult) (`.Location` (`GameplayStatics.BreakHitResult` _hitresult))))

(fn `DestroyCurrent`
  (bind _mesureactor (`self.MesureActor`))
  (`/Engine/EditorBlueprintResources/StandardMacros.IsValid` _mesureactor
    (:`Is Valid`
      (`self.K2_DestroyActor` _mesureactor))))

(fn `ProcessType`
  (params (Selection :type "/MyCustomWidget/Measure/BPE_MeasureType Enum" :default "NewEnumerator0"))
  (switch `/MyCustomWidget/Measure/BPE_MeasureType` Selection
    (:`NewEnumerator0`
      (`self.DestroyCurrent`)
      (message `/Game/Blueprints/Frame/BPI_PawnState.SetPawnState` (`GameplayStatics.GetPlayerPawn` 0) "NewEnumerator0"))
    (:`NewEnumerator1`
      (`self.DestroyCurrent`)
      (bind _returnvalue (`|SpawnActorFromClass` "/MyCustomWidget/Measure/Line/BP_MeasureActor_Linear.BP_MeasureActor_Linear_C" (`KismetMathLibrary.MakeTransform` (0.0 0.0 0.0)) "Undefined" "OverrideRootScale" null null))
      (set `self.MesureActor` _returnvalue)
      (message `/Game/Blueprints/Frame/BPI_PawnState.SetPawnState` (`GameplayStatics.GetPlayerPawn` 0) "NewEnumerator1"))
    (:`NewEnumerator2`
      (`self.DestroyCurrent`)
      (bind _returnvalue_2 (`|SpawnActorFromClass` "/MyCustomWidget/Measure/Area/BP_MeasureActor_Area.BP_MeasureActor_Area_C" (`KismetMathLibrary.MakeTransform` (0.0 0.0 0.0)) "Undefined" "OverrideRootScale" null null))
      (set `self.MesureActor` _returnvalue_2)
      (message `/Game/Blueprints/Frame/BPI_PawnState.SetPawnState` (`GameplayStatics.GetPlayerPawn` 0) "NewEnumerator1"))))

(fn `UserConstructionScript`)