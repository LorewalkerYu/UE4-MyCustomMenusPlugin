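; BP_MeasureActor_Linear is a linear measurement actor that traces a measured line with a spline.
; On BeginPlay it creates a widget set to metres, with a scale converting from centimetres.
; SetLastLocation moves the last spline point to a world location, or appends one when the spline has at most one point.
; AddLoacation is an empty event, and Tick only calls the parent.
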(event `self.ReceiveBeginPlay`
  (`self.CreateWidget` "米" 0.01))

(event `self.ReceiveTick`
  (params (DeltaSeconds :type "Float (single-precision)"))
  (`parent.ReceiveTick` DeltaSeconds))

(event `self.SetLastLocation`
  (params (LocationWS :type "Vector Structure"))
  (bind _spline (`self.Spline`))
  (bind _spline_2 (`self.Spline`))
  (if (<= (`SplineComponent.GetNumberOfSplinePoints` _spline) 1)
    (`SplineComponent.AddSplinePoint` _spline LocationWS "World" true)
    (else
      (`SplineComponent.SetLocationAtSplinePoint` _spline_2 (- (`SplineComponent.GetNumberOfSplinePoints` _spline_2) 1) LocationWS "World" true))))

(event `self.AddLoacation`
  (params (LocationWS :type "Vector Structure")))

(fn `UserConstructionScript`
  (`parent.UserConstructionScript`))