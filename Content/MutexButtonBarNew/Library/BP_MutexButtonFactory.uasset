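; Factory library that creates button widgets for the mutex button bar UI.
; Four functions build normal, color-change, floating-text and scalable floating-text variants, each layering more features on the last.
; Each maps info structs for initialization, color, scale or text onto widget creation inputs, then applies checkbox style and any text before returning the widget.
; Unlike the others, the plain color-change constructor takes no owning player.
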(fn `ConstructCorlorChangeButton`
  (params (InitializeInfo :type "/MyCustomWidget/MutexButtonBarNew/Button/BPF_ButtonInitizeInfo Structure") (ColorChangeInfo :type "/MyCustomWidget/MutexButtonBarNew/Button/BPF_ColorChangeInfo Structure"))
  (returns (ConstructedButton :type "/MyCustomWidget/MutexButtonBarNew/WBP_Button_Base Object Reference"))
  (bind (_displaywidget _id _bstartwithdisabled _bstartchecked _maximumsize _checkboxstyle) (break `/MyCustomWidget/MutexButtonBarNew/Button/BPF_ButtonInitizeInfo` InitializeInfo))
  (bind (_normalcolor _checkedcolor) (break `/MyCustomWidget/MutexButtonBarNew/Button/BPF_ColorChangeInfo` ColorChangeInfo))
  (bind _returnvalue (`|CreateWidget` "/MyCustomWidget/MutexButtonBarNew/Button/WBP_Button_ColorChange.WBP_Button_ColorChange_C" null _normalcolor _checkedcolor _displaywidget _id _bstartwithdisabled _bstartchecked _maximumsize))
  (`/MyCustomWidget/MutexButtonBarNew/WBP_Button_Base.SetCheckBoxStyle` _returnvalue _checkboxstyle)
  (return _returnvalue))

(fn `ConstructCorlorChangeButton_FloatingText`
  (params (OwningPlayer :type "PlayerController Object Reference") (InitializeInfo :type "/MyCustomWidget/MutexButtonBarNew/Button/BPF_ButtonInitizeInfo Structure") (ColorChangeInfo :type "/MyCustomWidget/MutexButtonBarNew/Button/BPF_ColorChangeInfo Structure") (FloatingTextInfo :type "/MyCustomWidget/MutexButtonBarNew/Button/BPF_FloatingTextInfo Structure"))
  (returns (ConstructedButton :type "/MyCustomWidget/MutexButtonBarNew/WBP_Button_Base Object Reference"))
  (bind (_displaywidget _id _bstartwithdisabled _bstartchecked _maximumsize _checkboxstyle) (break `/MyCustomWidget/MutexButtonBarNew/Button/BPF_ButtonInitizeInfo` InitializeInfo))
  (bind (_normalcolor _checkedcolor) (break `/MyCustomWidget/MutexButtonBarNew/Button/BPF_ColorChangeInfo` ColorChangeInfo))
  (bind (_text _offset _font) (break `/MyCustomWidget/MutexButtonBarNew/Button/BPF_FloatingTextInfo` FloatingTextInfo))
  (bind _returnvalue (`|CreateWidget` "/MyCustomWidget/MutexButtonBarNew/Button/WBP_Button_ColorChange_FloatingText.WBP_Button_ColorChange_FloatingText_C" OwningPlayer _normalcolor _checkedcolor _displaywidget _id _bstartwithdisabled _bstartchecked _maximumsize))
  (`/MyCustomWidget/MutexButtonBarNew/WBP_Button_Base.SetCheckBoxStyle` _returnvalue _checkboxstyle)
  (`/MyCustomWidget/MutexButtonBarNew/Button/WBP_Button_ColorChange_FloatingText.SetText` _returnvalue _text _font)
  (return _returnvalue))

(fn `ConstructCorlorChangeButton_FloatingText_Scaleable`
  (params (OwningPlayer :type "PlayerController Object Reference") (InitializeInfo :type "/MyCustomWidget/MutexButtonBarNew/Button/BPF_ButtonInitizeInfo Structure") (ScaleableInfo :type "/MyCustomWidget/MutexButtonBarNew/Button/BPF_Scaleablenfo Structure") (ColorChangeInfo :type "/MyCustomWidget/MutexButtonBarNew/Button/BPF_ColorChangeInfo Structure") (FloatingTextInfo :type "/MyCustomWidget/MutexButtonBarNew/Button/BPF_FloatingTextInfo Structure"))
  (returns (ConstructedButton :type "/MyCustomWidget/MutexButtonBarNew/WBP_Button_Base Object Reference"))
  (bind (_displaywidget _id _bstartwithdisabled _bstartchecked _maximumsize _checkboxstyle) (break `/MyCustomWidget/MutexButtonBarNew/Button/BPF_ButtonInitizeInfo` InitializeInfo))
  (bind (_normalcolor _checkedcolor) (break `/MyCustomWidget/MutexButtonBarNew/Button/BPF_ColorChangeInfo` ColorChangeInfo))
  (bind (_text _offset _font) (break `/MyCustomWidget/MutexButtonBarNew/Button/BPF_FloatingTextInfo` FloatingTextInfo))
  (bind (_normalscale _checkedscale) (break `/MyCustomWidget/MutexButtonBarNew/Button/BPF_Scaleablenfo` ScaleableInfo))
  (bind _returnvalue (`|CreateWidget` "/MyCustomWidget/MutexButtonBarNew/Button/WBP_Button_ColorChange_FloatingText_Scaleble.WBP_Button_ColorChange_FloatingText_Scaleble_C" OwningPlayer _normalcolor _checkedcolor _normalscale _checkedscale _displaywidget _id _bstartwithdisabled _bstartchecked _maximumsize))
  (`/MyCustomWidget/MutexButtonBarNew/WBP_Button_Base.SetCheckBoxStyle` _returnvalue _checkboxstyle)
  (`/MyCustomWidget/MutexButtonBarNew/Button/WBP_Button_ColorChange_FloatingText_Scaleble.SetFloatingText` _returnvalue _text _offset _font)
  (return _returnvalue))

(fn `ConstructNormalButton`
  (params (OwningPlayer :type "PlayerController Object Reference") (InitializeInfo :type "/MyCustomWidget/MutexButtonBarNew/Button/BPF_ButtonInitizeInfo Structure"))
  (returns (ConstructedButton :type "/MyCustomWidget/MutexButtonBarNew/WBP_Button_Base Object Reference"))
  (bind (_displaywidget _id _bstartwithdisabled _bstartchecked _maximumsize _checkboxstyle) (break `/MyCustomWidget/MutexButtonBarNew/Button/BPF_ButtonInitizeInfo` InitializeInfo))
  (bind _returnvalue (`|CreateWidget` "/MyCustomWidget/MutexButtonBarNew/Button/WBP_Button_Normal.WBP_Button_Normal_C" OwningPlayer _displaywidget _id _bstartwithdisabled _bstartchecked _maximumsize))
  (`/MyCustomWidget/MutexButtonBarNew/Button/WBP_Button_Normal.SetCheckBoxStyle` _returnvalue _checkboxstyle)
  (return _returnvalue))