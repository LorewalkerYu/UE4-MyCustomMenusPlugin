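; Function library that builds display widgets for the Mutex button bar UI.
; Each function creates one widget type: text with font and color, texture image, image downloaded from a URL at a given size, or image with text.
; Inputs are passed at widget creation, except the image-with-text caption, which is set on its Text child afterward, and the new widget is returned.
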(fn `ConstructMutexDownloadImageDisplay`
  (params (ImageURL :type String) (Size :type "Vector2D Structure"))
  (returns (ReturnValue :type "/MyCustomWidget/MutexButtonBarNew/Display/WBP_Display_DownloadImage Object Reference"))
  (bind _returnvalue (`|CreateWidget` "/MyCustomWidget/MutexButtonBarNew/Display/WBP_Display_DownloadImage.WBP_Display_DownloadImage_C" null Size ImageURL))
  (return _returnvalue))

(fn `ConstructMutexImageDisplay`
  (params (Texture :type "Texture2D Object Reference"))
  (returns (ReturnValue :type "/MyCustomWidget/MutexButtonBarNew/Display/WBP_Display_Image Object Reference"))
  (bind _returnvalue (`|CreateWidget` "/MyCustomWidget/MutexButtonBarNew/Display/WBP_Display_Image.WBP_Display_Image_C" null Texture))
  (return _returnvalue))

(fn `ConstructMutexImageTextDisplay`
  (params (Texture :type "Texture2D Object Reference") (InText :type Text))
  (returns (ReturnValue :type "/MyCustomWidget/MutexButtonBarNew/WBP_ButtonDisplay_Base Object Reference"))
  (bind _returnvalue (`|CreateWidget` "/MyCustomWidget/MutexButtonBarNew/Display/WBP_Display_Image_Text.WBP_Display_Image_Text_C" null Texture))
  (`TextBlock.SetText` (`/MyCustomWidget/MutexButtonBarNew/Display/WBP_Display_Image_Text.Text` _returnvalue) InText)
  (return _returnvalue))

(fn `ConstructMutexTextDisplay`
  (params (DisplayText :type Text) (Font :type "SlateFontInfo Structure") (Color :type "/MyCustomWidget/MutexButtonBarNew/Button/BPF_ColorChangeInfo Structure"))
  (returns (ReturnValue :type "/MyCustomWidget/MutexButtonBarNew/Display/WBP_Display_Text Object Reference"))
  (bind _returnvalue (`|CreateWidget` "/MyCustomWidget/MutexButtonBarNew/Display/WBP_Display_Text.WBP_Display_Text_C" null DisplayText Font Color))
  (return _returnvalue))